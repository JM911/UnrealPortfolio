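; BP_Enemy_Default is an enemy Blueprint that displays a floating HP bar through its EnemyWidget component.
; BeginPlay caches the component's WBP_EnemyUI instance.
; Each Tick, it sets the bar from CurrentHp over MaxHp and billboards the widget by inverting camera pitch and turning yaw 180 degrees.
; Tick also shows the UI only while the player pawn is within WidgetVisibleDistance.
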(event EventBeginPlay
  (bind _aswbp_enemy_ui (Utilities|Casting|CastToWBP_EnemyUI (UserInterface|GetUserWidgetObject (Variables|Default|GetEnemy%20Widget))))
  (Variables|Default|SetEnemyUIRef _aswbp_enemy_ui))

(event Collision|EventActorBeginOverlap
  (params (OtherActor :type Actor%20Object%20Reference)))

(event EventTick
  (params (DeltaSeconds :type Float%20%28single-precision%29))
  (bind _returnvalue (Game|GetPlayerController 0))
  (bind _playercameramanager (Variables|/Script/Engine.PlayerController|GetPlayerCameraManager _returnvalue))
  (bind _returnvalue_2 (Transformation|GetActorRotation _playercameramanager))
  (Utilities|FlowControl|Sequence
    (:then_0
      (Progress|SetPercent (Variables|/Game/_LootAndShoot/Blueprints/WBP_EnemyUI.WBP_EnemyUI_C|GetEnemyHpBar (Variables|Default|GetEnemyUIRef)) (/ (Variables|Default|GetCurrentHp) (Variables|Default|GetMaxHp))))
    (:then_1
      (Transformation|SetWorldRotation (Variables|Default|GetEnemy%20Widget) (Math|Rotator|MakeRotator 0.0 (* (.pitch _returnvalue_2) -1.0) (+ (.yaw _returnvalue_2) 1.8e+02)) false false))
    (:then_2
      (if (< (Math|Vector|Distance(Vector) (Transformation|GetActorLocation (Game|Player|GetPlayerPawn 0)) (Transformation|GetActorLocation)) (Variables|Default|GetWidgetVisibleDistance))
        (Widget|SetVisibility (Variables|Default|GetEnemyUIRef) "Visible")
        (else
          (Widget|SetVisibility (Variables|Default|GetEnemyUIRef) "Hidden"))))))

(fn ConstructionScript)